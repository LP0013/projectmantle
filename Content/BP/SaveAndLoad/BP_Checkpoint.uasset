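; BP_Checkpoint is a side-scroller checkpoint that saves the game and opens a checkpoint menu when the player presses Interact within its Box.
; Box overlaps toggle the actor's input and open or close a Gate for SideScrollerCharacter, with a short delay on exit.
; Interact passes through the Gate to show CheckpointMenu with UI-only input and a visible cursor, then saves the character to slot "Save1".
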(event OnComponentBeginOverlap(Box)
  (params (OverlappedComponent :type Primitive%20Component%20Object%20Reference) (OtherActor :type Actor%20Object%20Reference) (OtherComp :type Primitive%20Component%20Object%20Reference) (OtherBodyIndex :type Integer) (bFromSweep :type Boolean) (SweepResult :type Hit%20Result%20Structure%20%28by%20ref%29))
  (bind _returnvalue (Game|GetPlayerController 0))
  (Input|EnableInput (Game|GetPlayerController 0))
  (Utilities|Casting|CastToSideScrollerCharacter OtherActor)
  (Utilities|FlowControl|Gate true) ; enters at Open
)

(event OnComponentEndOverlap(Box)
  (params (OverlappedComponent :type Primitive%20Component%20Object%20Reference) (OtherActor :type Actor%20Object%20Reference) (OtherComp :type Primitive%20Component%20Object%20Reference) (OtherBodyIndex :type Integer))
  (bind _returnvalue (Game|GetPlayerController 0))
  (Utilities|FlowControl|Delay 0.2)
  (Input|DisableInput (Game|GetPlayerController 0) 0)
  (Utilities|Casting|CastToSideScrollerCharacter OtherActor)
  (Utilities|FlowControl|Gate true) ; enters at Close
)

(event Input|ActionEvents|InputActionInteract
  (params (Key :type Key%20Structure :default "None"))
  (bind _returnvalue (Game|GetPlayerController 0))
  (:Pressed
    (Utilities|FlowControl|Gate true
      (:Exit
        (bind _asside_scroller_character (Utilities|Casting|CastToSideScrollerCharacter (Game|GetPlayerCharacter 0)))
        (bind _returnvalue_2 (UserInterface|CreateWidget "/Game/UI/CheckpointMenu.CheckpointMenu_C"))
        (UserInterface|Viewport|AddtoViewport _returnvalue_2 0)
        (Input|SetInputModeUIOnly _returnvalue 0 "LockAlways")
        (Variables|/Script/Engine.PlayerController|SetbShowMouseCursor _returnvalue true)
        (Default|SaveGame _asside_scroller_character "Save1")
        (Development|PrintString "SAved")))))

(fn ConstructionScript)