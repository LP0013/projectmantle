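; BP_WaterArea is a water volume that hampers the side-scroller character's movement.
; Entering its Box removes the extra jump, disables levitation, and lowers walk speed and dash distance.
; Leaving starts a five-second Delay, then sets those properties to hardcoded normal values rather than saved originals.
; The delayed reset does not check whether the character has re-entered the water.
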(event OnComponentBeginOverlap(Box)
  (params (OverlappedComponent :type Primitive%20Component%20Object%20Reference) (OtherActor :type Actor%20Object%20Reference) (OtherComp :type Primitive%20Component%20Object%20Reference) (OtherBodyIndex :type Integer) (bFromSweep :type Boolean) (SweepResult :type Hit%20Result%20Structure%20%28by%20ref%29))
  ;[0.08138 0.05392 1] WaterAreaStart
  (bind _asside_scroller_character (Utilities|Casting|CastToSideScrollerCharacter OtherActor))
  (Variables|/Script/Engine.Character|SetJumpMaxCount _asside_scroller_character 1)
  (Variables|/Game/SideScrollerBP/Blueprints/SideScrollerCharacter.SideScrollerCharacter_C|SetShouldLevitate _asside_scroller_character false)
  (Variables|/Script/Engine.CharacterMovementComponent|SetMaxWalkSpeed (Variables|/Script/Engine.Character|GetCharacterMovement _asside_scroller_character) 1e+02)
  (Variables|/Game/SideScrollerBP/Blueprints/SideScrollerCharacter.SideScrollerCharacter_C|SetDashDistance _asside_scroller_character 4e+03))

(event OnComponentEndOverlap(Box)
  (params (OverlappedComponent :type Primitive%20Component%20Object%20Reference) (OtherActor :type Actor%20Object%20Reference) (OtherComp :type Primitive%20Component%20Object%20Reference) (OtherBodyIndex :type Integer))
  ;[1 0.2252 0.1754] WaterAreaEnd
  (Utilities|FlowControl|Delay 5.0)
  (bind _asside_scroller_character (Utilities|Casting|CastToSideScrollerCharacter OtherActor))
  (Variables|/Script/Engine.Character|SetJumpMaxCount _asside_scroller_character 2)
  (Variables|/Game/SideScrollerBP/Blueprints/SideScrollerCharacter.SideScrollerCharacter_C|SetShouldLevitate _asside_scroller_character true)
  (Variables|/Script/Engine.CharacterMovementComponent|SetMaxWalkSpeed (Variables|/Script/Engine.Character|GetCharacterMovement _asside_scroller_character) 1e+03)
  (Variables|/Game/SideScrollerBP/Blueprints/SideScrollerCharacter.SideScrollerCharacter_C|SetDashDistance _asside_scroller_character 6e+03))

(fn ConstructionScript)