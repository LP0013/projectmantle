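; BP_floorFan is a side-scroller floor fan that blows the player along its Arrow and can be briefly switched off.
; Any overlap with Box launches player 0; the SideScrollerCharacter also gets negative gravity and shorter dash distance until leaving.
; Box1 shows an interact widget, enables input and opens a gate, which is never closed.
; Interact then hides Box and disables its collision and tick, restoring them after a delay.
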(event OnComponentEndOverlap(Box1)
  (params (OverlappedComponent :type Primitive%20Component%20Object%20Reference) (OtherActor :type Actor%20Object%20Reference) (OtherComp :type Primitive%20Component%20Object%20Reference) (OtherBodyIndex :type Integer))
  ;[1 1 1] Enable Disable Fan
  (Widget|RemovefromParent (stale OnComponentBeginOverlap(Box1) _returnvalue)))

(event OnComponentBeginOverlap(Box1)
  (params (OverlappedComponent :type Primitive%20Component%20Object%20Reference) (OtherActor :type Actor%20Object%20Reference) (OtherComp :type Primitive%20Component%20Object%20Reference) (OtherBodyIndex :type Integer) (bFromSweep :type Boolean) (SweepResult :type Hit%20Result%20Structure%20%28by%20ref%29))
  (bind _box (Variables|Default|GetBox))
  ;[1 1 1] Enable Disable Fan
  (Input|EnableInput (Game|GetPlayerController 0))
  (bind _returnvalue (UserInterface|CreateWidget "/Game/UI/InteractWidg.InteractWidg_C"))
  (UserInterface|Viewport|AddtoViewport _returnvalue 0)
  (Utilities|Casting|CastToSideScrollerCharacter OtherActor)
  (Utilities|FlowControl|Gate true) ; enters at Open
)

(event OnComponentBeginOverlap(Box)
  (params (OverlappedComponent :type Primitive%20Component%20Object%20Reference) (OtherActor :type Actor%20Object%20Reference) (OtherComp :type Primitive%20Component%20Object%20Reference) (OtherBodyIndex :type Integer) (bFromSweep :type Boolean) (SweepResult :type Hit%20Result%20Structure%20%28by%20ref%29))
  (Character|LaunchCharacter (Game|GetPlayerCharacter 0) (* (Math|Vector|GetForwardVector (Variables|Default|GetArrow)) 1e+03) true true)
  (bind _asside_scroller_character (Utilities|Casting|CastToSideScrollerCharacter OtherActor))
  (Variables|/Script/Engine.CharacterMovementComponent|SetGravityScale (Variables|/Script/Engine.Character|GetCharacterMovement _asside_scroller_character) -0.6)
  ;[1 1 1] Dash Distancs on fan
  (Variables|/Game/SideScrollerBP/Blueprints/SideScrollerCharacter.SideScrollerCharacter_C|SetDashDistance _asside_scroller_character 2e+03))

(event OnComponentEndOverlap(Box)
  (params (OverlappedComponent :type Primitive%20Component%20Object%20Reference) (OtherActor :type Actor%20Object%20Reference) (OtherComp :type Primitive%20Component%20Object%20Reference) (OtherBodyIndex :type Integer))
  (bind _asside_scroller_character (Utilities|Casting|CastToSideScrollerCharacter OtherActor))
  (Variables|/Script/Engine.CharacterMovementComponent|SetGravityScale (Variables|/Script/Engine.Character|GetCharacterMovement _asside_scroller_character) 2.0)
  ;[1 1 1] Dash Distancs on fan
  (Variables|/Game/SideScrollerBP/Blueprints/SideScrollerCharacter.SideScrollerCharacter_C|SetDashDistance _asside_scroller_character 6e+03))

(event Input|ActionEvents|InputActionInteract
  (params (Key :type Key%20Structure :default "None"))
  (bind _box (Variables|Default|GetBox))
  ;[1 1 1] Enable Disable Fan
  (:Pressed
    (Utilities|FlowControl|Gate true
      (:Exit
        (Utilities|Casting|CastToSideScrollerCharacter (Game|GetPlayerCharacter 0))
        (Rendering|SetVisibility _box false false)
        (Collision|SetCollisionEnabled _box "NoCollision")
        (Components|Tick|SetComponentTickEnabled _box false)
        (Utilities|FlowControl|Delay 3.0)
        (Rendering|SetVisibility _box true false)
        (Collision|SetCollisionEnabled _box "QueryAndPhysics")
        (Components|Tick|SetComponentTickEnabled _box true)))))

(fn ConstructionScript)